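; BP_ShieldEffect is a shield effect actor that follows a character and toggles its sprite collision and particle visual on activation and deactivation.
; OnActiveEffect attaches the actor to the given Character, zeroes its relative location, switches the PaperSprite to OverlapAll collision and spawns the Main_defense emitter on the Character's root.
; OnDeActiveEffect sets the sprite to NoCollision and destroys the stored particle, leaving the actor attached.
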(event `self.ReceiveBeginPlay`)

(event `self.BP_OnActiveEffect`
  (params (Character :type "Character Object Reference"))
  (`self.K2_AttachToActor` Character "None" "KeepRelative" "KeepRelative" "KeepRelative")
  (`self.K2_SetActorRelativeLocation` (0.0 0.0 0.0))
  (`PrimitiveComponent.SetCollisionProfileName` (`self.PaperSprite`) "OverlapAll" true)
  (bind _returnvalue (`GameplayStatics.SpawnEmitterAttached` "/Game/FX/Jlingchen/Main_defense.Main_defense" (`Actor.RootComponent` Character)))
  (set `self.Particle` _returnvalue))

(event `self.BP_OnDeActiveEffect`
  (params (Character :type "Character Object Reference"))
  (`PrimitiveComponent.SetCollisionProfileName` (`self.PaperSprite`) "NoCollision" true)
  (`ActorComponent.K2_DestroyComponent` (`self.Particle`)))

(fn `UserConstructionScript`)