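; BP_Arrow is a side-scroller projectile that the player can deflect by attacking.
; Sprite overlap casts pick the outcome: damage to player or AI, shield or fireball impact, or deactivation on other surfaces; spikeweed and arrows are ignored.
; A deflect updates the player's combo count and dispatchers, plays a sound, and stops ProjectileMovement.
; Tick then moves the flipped arrow along a fixed local direction; boss-aiming code is unconnected.
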(event `self.ReceiveBeginPlay`
  (`self.K2_SetActorRotation` (`KismetMathLibrary.MakeRotator` 0.0 30.0)))

(event `self.ReceiveTick`
  (params (DeltaSeconds :type "Float (single-precision)"))
  (if (`self.IsRebound`)
    (`self.K2_AddActorLocalOffset` (* (`self.Direction`) (* DeltaSeconds (`self.Speed`))))))

(event `self.PaperSprite.OnComponentBeginOverlap`
  (params (OverlappedComponent :type "PrimitiveComponent Object Reference") (OtherActor :type "Actor Object Reference") (OtherComp :type "PrimitiveComponent Object Reference") (OtherBodyIndex :type Integer) (bFromSweep :type Boolean) (SweepResult :type "HitResult Structure (by ref)"))
  (bind _audio (`self.Audio`))
  (bind _asbp_2dside_scroller_character (cast `/Game/Blueprints/BP_2DSideScrollerCharacter` OtherActor)
    (:`then`
      (if (`SwordRetaliateCharacter.IsCharacterAttackAction` _asbp_2dside_scroller_character)
        (`GameplayStatics.SpawnEmitterAtLocation` "/Game/FX/Jlingchen/Main_hit.Main_hit" (`self.K2_GetActorLocation`) (struct) (1.2 1.2 1.2))
        (bind _returnvalue (+ (`/Game/Blueprints/BP_2DSideScrollerCharacter.Cnt` _asbp_2dside_scroller_character) 1))
        (bind _output_get (set `/Game/Blueprints/BP_2DSideScrollerCharacter.Cnt` _returnvalue _asbp_2dside_scroller_character))
        (`/Game/Blueprints/BP_2DSideScrollerCharacter.ScoreDispatcher` _asbp_2dside_scroller_character _output_get)
        (`|ExecutionSequence`
          (:`then_0`
            (`ActorComponent.Deactivate` (`self.ProjectileMovement`))
            (`ActorComponent.Activate` (`self.Audio`) false)
            (`AudioComponent.SetSound` _audio "/Game/Music/TANFAN.TANFAN")
            (`AudioComponent.Play` _audio 0.0)
            (set `self.Direction` (1.0 0.0 0.0))
            (set `self.IsRebound` true)
            (`self.K2_SetActorRotation` (struct :`Pitch` 180.0)))
          (:`then_1`
            (bind _output_get_2 (set `self.Pawn` _asbp_2dside_scroller_character))
            (`/Game/Blueprints/BP_2DSideScrollerCharacter.AddPersentDispatcher` _output_get_2 0.02)
            (bind _maxcnt (`/Game/Blueprints/BP_2DSideScrollerCharacter.MaxCnt` _output_get_2))
            (if (> _returnvalue _maxcnt)
              (set `/Game/Blueprints/BP_2DSideScrollerCharacter.MaxCnt` _maxcnt _output_get_2)
              (set `/Game/Blueprints/BP_2DSideScrollerCharacter.Score` (+ _returnvalue (`/Game/Blueprints/BP_2DSideScrollerCharacter.Score` _output_get_2)) _output_get_2))))
        (else
          (`SwordRetaliateCharacter.OnCharacterHit` _asbp_2dside_scroller_character 10.0)
          (set `/Game/Blueprints/BP_2DSideScrollerCharacter.Cnt` 0 _asbp_2dside_scroller_character)
          (`self.SpawnParticleAndDestroy` "/Game/FX/FX_HitCharacter.FX_HitCharacter"))))
    (:`CastFailed`
      (bind _assword_retaliate_aicharacter (cast `/Game/2DSideScroller/AI/SwordRetaliateAICharacter` OtherActor)
        (:`then`
          (`/Game/2DSideScroller/AI/SwordRetaliateAICharacter.OnAIHit` _assword_retaliate_aicharacter 1.0)
          (`self.SpawnParticleAndDestroy` "/Game/FX/FX_HitCharacter.FX_HitCharacter"))
        (:`CastFailed`
          (bind _asbp_shield_effect (cast `/Game/Blueprints/BP_ShieldEffect` OtherActor)
            (:`then`
              (`AudioComponent.Play` (`/Game/Blueprints/BP_ShieldEffect.Audio` _asbp_shield_effect) 0.0)
              (`self.SpawnParticleAndDestroy` "/Game/FX/FX_HitShield.FX_HitShield"))
            (:`CastFailed`
              (cast `/Game/Blueprints/BP_FireEffect` OtherActor
                (:`then`
                  (`self.SpawnParticleAndDestroy` "/Game/FX/FX_FireBallHit.FX_FireBallHit"))
                (:`CastFailed`
                  (cast `/Game/Blueprints/Scene/BP_Spikeweed` OtherActor
                    (:`CastFailed`
                      (cast `/Game/Blueprints/Scene/BP_Arrow` OtherActor
                        (:`CastFailed`
                          (`self.Spawn Particle and Deactivate` "/Game/FX/FX_HitGrass.FX_HitGrass"))))))))))))))

(fn `Spawn Particle and Deactivate`
  (params (Particle :type "ParticleSystem Object Reference"))
  (`GameplayStatics.SpawnEmitterAtLocation` Particle (`SceneComponent.K2_GetComponentLocation` (`self.Sphere`)))
  (`ActorComponent.Deactivate` (`self.ProjectileMovement`))
  (`PrimitiveComponent.SetCollisionProfileName` (`self.PaperSprite`) "NoCollision" true))

(fn `SpawnParticleAndDestroy`
  (params (Particle :type "ParticleSystem Object Reference"))
  (`GameplayStatics.SpawnEmitterAtLocation` Particle (`SceneComponent.K2_GetComponentLocation` (`self.Sphere`)))
  (`self.K2_DestroyActor`))

(fn `UserConstructionScript`)