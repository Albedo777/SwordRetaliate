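; Rhythm-style arrow generator that plays the LoudnessAnalyzer's sound and spawns an actor at its own location on loudness peaks.
; Playback-percent updates advance a timer in audio time, running a peak check each time the CD cooldown elapses.
; SampleFunc detects peaks by comparing loudness to samples about 0.1s either side, within a loudness band.
; Its two song-range checks join bounds with OR, so they barely restrict position.
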(event `self.ReceiveBeginPlay`
  (set `self.ZHeight` (.z (`self.K2_GetActorLocation`)))
  (add `AudioComponent.OnAudioPlaybackPercent` (`self.Audio`) (delegate `PlaybackPercentEvent`))
  (`AudioComponent.Play` (`self.Audio`) 0.0)
  (bind _isspawn (`self.SampleFunc` (stale `PlaybackPercentEvent` PlaybackPercent) (`self.Duration`) 0.0 0.642 (`self.LastPercent`) 0.0 1.0 :!label _label))
  (if _isspawn
    (`|SpawnActorFromClass` "/Game/Blueprints/Scene/BP_Arrow.BP_Arrow_C" (`KismetMathLibrary.Conv_VectorToTransform` (`KismetMathLibrary.MakeVector` (.x (`self.K2_GetActorLocation`)) (.y (`self.K2_GetActorLocation`)) (`self.ZHeight`))) "Undefined" "OverrideRootScale" null null :!label _label_2)
    (else
      (bind _isspawn_2 (`self.SampleFunc` (stale `PlaybackPercentEvent` PlaybackPercent) (`self.Duration`) 0.765 1.0 (`self.LastPercent`) 0.0 1.0))
      (if _isspawn_2
        (goto _label_2)))))

(event `PlaybackPercentEvent`
  (params (PlayingSoundWave :type "SoundWave Object Reference") (PlaybackPercent :type "Float (double-precision)"))
  (bind _output_get (set `self.Timer` (+ (* (- PlaybackPercent (`self.LastPercent`)) (`self.Duration`)) (`self.Timer`))))
  (set `self.LastPercent` PlaybackPercent)
  (if (> _output_get (`self.CD`))
    (set `self.Timer` 0.0)
    (goto _label)))

(event `InputAction|Print`
  (params (Key :type "Key Structure"))
  (:`Pressed`
    (`KismetSystemLibrary.PrintString` (`KismetStringLibrary.Concat_StrStr` (`KismetStringLibrary.Conv_DoubleToString` (`self.LastPercent`)) "percent"))))

(fn `SampleFunc`
  (params (PlayPercent :type "Float (double-precision)") (Duration :type "Float (double-precision)") (SampleStart :type "Float (double-precision)") (SampleEnd :type "Float (double-precision)") (LastPercent :type "Float (double-precision)") (LoudnessLow :type "Float (double-precision)") (LoudnessHigh :type "Float (double-precision)"))
  (returns (ISSpawn :type Boolean))
  (bind _returnvalue (* PlayPercent Duration))
  (bind _outloudness (`LoudnessNRT.GetNormalizedChannelLoudnessAtTime` (`self.LoudnessAnalyzer`) _returnvalue 0))
  (if (> _outloudness (`LoudnessNRT.GetNormalizedChannelLoudnessAtTime` (`self.LoudnessAnalyzer`) (- _returnvalue 0.10132) 0))
    (if (> _outloudness (`LoudnessNRT.GetNormalizedChannelLoudnessAtTime` (`self.LoudnessAnalyzer`) (+ _returnvalue 0.10132) 0))
      (if (or (> LastPercent SampleStart) (< LastPercent SampleEnd))
        (if (and (> _outloudness LoudnessLow) (< _outloudness LoudnessHigh))
          (`KismetSystemLibrary.PrintString` (`KismetStringLibrary.Conv_DoubleToString` _outloudness))
          (return true)
          (else
            _)))))
  (return false))

(fn `UserConstructionScript`
  (bind _sound (`AudioAnalyzerNRT.Sound` (`self.LoudnessAnalyzer`)))
  ;[1 1 1] Get Sound From Loudness Analyze
  (`AudioComponent.SetSound` (`self.Audio`) _sound)
  ;[1 1 1] Store Sound Duration
  (set `self.Duration` (`SoundBase.Duration` _sound)))