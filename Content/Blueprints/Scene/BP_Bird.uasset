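; BP_Bird is a scene actor that shows a bird as a Paper2D flipbook flying along positive X with a wandering height.
; Tick accumulates a timer and every half second calls UpdateDirection, which keeps forward X fixed and randomizes a small up or down Z component.
; Each frame it offsets the flipbook component, not the actor, by that direction scaled by Speed and delta time, without sweeping.
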(event `self.ReceiveTick`
  (params (DeltaSeconds :type "Float (single-precision)"))
  (bind _output_get (set `self.Timer` (+ DeltaSeconds (`self.Timer`))))
  (if (>= _output_get 0.5)
    (set `self.Timer` 0.0)
    (bind _direction (`self.UpdateDirection`))
    (set `self.Dir` _direction))
  (`SceneComponent.K2_AddWorldOffset` (`self.PaperFlipbook`) (* (`self.Dir`) (* DeltaSeconds (`self.Speed`))) false false))

(fn `UpdateDirection`
  (returns (Direction :type "Vector Structure"))
  (return (`KismetMathLibrary.MakeVector` (.x (1.0 0.0 1.0)) (.y (1.0 0.0 1.0)) (* (.z (1.0 0.0 1.0)) (`KismetMathLibrary.RandomFloatInRange` -0.4 0.4)))))

(fn `UserConstructionScript`)