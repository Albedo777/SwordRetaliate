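; BP_Spikeweed is a spike trap that pops up when the player character approaches and hurts it on contact.
; Overlapping the probe sprite sets MoveFlag, so Tick moves the actor along local up by Speed each frame, unscaled by delta time, until LimitTime runs out.
; The main sprite's overlap calls OnCharacterHit on SwordRetaliateCharacter with fixed damage and spawns a hit effect.
; Destruction also calls an emitter spawn, with no template shown.
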(event `self.ReceiveTick`
  (params (DeltaSeconds :type "Float (single-precision)"))
  (if (`self.MoveFlag`)
    (`self.UpdateLocation` DeltaSeconds)))

(event `self.PaperSprite.OnComponentBeginOverlap`
  (params (OverlappedComponent :type "PrimitiveComponent Object Reference") (OtherActor :type "Actor Object Reference") (OtherComp :type "PrimitiveComponent Object Reference") (OtherBodyIndex :type Integer) (bFromSweep :type Boolean) (SweepResult :type "HitResult Structure (by ref)"))
  (bind _assword_retaliate_character (cast `SwordRetaliateCharacter` OtherActor))
  (`SwordRetaliateCharacter.OnCharacterHit` _assword_retaliate_character 10.0)
  (`GameplayStatics.SpawnEmitterAtLocation` "/Game/FX/Jlingchen/Main_hit.Main_hit" (`self.K2_GetActorLocation`) (struct) (1.2 1.2 1.2)))

(event `self.ReceiveDestroyed`
  (`GameplayStatics.SpawnEmitterAtLocation` null (`self.K2_GetActorLocation`)))

(event `self.PaperSpriteProbe.OnComponentBeginOverlap`
  (params (OverlappedComponent :type "PrimitiveComponent Object Reference") (OtherActor :type "Actor Object Reference") (OtherComp :type "PrimitiveComponent Object Reference") (OtherBodyIndex :type Integer) (bFromSweep :type Boolean) (SweepResult :type "HitResult Structure (by ref)"))
  (cast `SwordRetaliateCharacter` OtherActor)
  (set `self.MoveFlag` true))

(fn `UpdateLocation`
  (params (DeltaTime :type "Float (double-precision)"))
  (`self.K2_AddActorLocalOffset` (* (`KismetMathLibrary.Vector_Up`) (`self.Speed`)))
  (bind _output_get (set `self.LimitTime` (- (`self.LimitTime`) DeltaTime)))
  (if (<= _output_get 0.0)
    (set `self.MoveFlag` false)))

(fn `UserConstructionScript`)