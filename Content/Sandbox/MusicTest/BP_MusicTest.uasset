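; Music-reactive test actor that plays a track, pulses two spheres to its loudness, and spawns BP_Stone on loudness peaks.
; The construction script takes the sound and its duration from a LoudnessAnalyzer asset.
; Each playback-percent callback samples precomputed channel 0 loudness to scale and print.
; When the cooldown elapses, a stone spawns at a fixed point if loudness exceeds samples slightly before and after, using look-ahead into the analysis.
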(event `self.ReceiveBeginPlay`
  (add `AudioComponent.OnAudioPlaybackPercent` (`self.Audio`) (delegate `PlaybackPercentEvent`))
  (`AudioComponent.Play` (`self.Audio`) 0.0)
  (bind _returnvalue (* (stale `PlaybackPercentEvent` PlaybackPercent) (`self.Duration`)))
  (if (> (`LoudnessNRT.GetNormalizedChannelLoudnessAtTime` (`self.LoudnessAnalyzer`) _returnvalue 0) (`LoudnessNRT.GetNormalizedChannelLoudnessAtTime` (`self.LoudnessAnalyzer`) (+ _returnvalue 0.10132) 0)) :!label _label
    (`|SpawnActorFromClass` "/Game/Sandbox/MusicTest/BP_Stone.BP_Stone_C" (`KismetMathLibrary.MakeTransform` (0.0 400.0 0.0)) "Undefined" "OverrideRootScale" null null)))

(event `PlaybackPercentEvent`
  (params (PlayingSoundWave :type "SoundWave Object Reference") (PlaybackPercent :type "Float (double-precision)"))
  (bind _returnvalue (* PlaybackPercent (`self.Duration`)))
  (bind _returnvalue_2 (* PlaybackPercent (`self.Duration`)))
  (bind _outloudness (`LoudnessNRT.GetNormalizedChannelLoudnessAtTime` (`self.LoudnessAnalyzer`) _returnvalue_2 0))
  ;[1 1 1] sphere
  (`KismetSystemLibrary.PrintString` (`KismetStringLibrary.Conv_DoubleToString` _outloudness))
  (`SceneComponent.SetRelativeScale3D` (`self.LeftSphere`) (`KismetMathLibrary.Conv_DoubleToVector` _outloudness))
  (`SceneComponent.SetRelativeScale3D` (`self.RightSphere`) (`KismetMathLibrary.Conv_DoubleToVector` (`LoudnessNRT.GetNormalizedChannelLoudnessAtTime` (`self.LoudnessAnalyzer`) _returnvalue_2 0)))
  (bind _output_get (set `self.Timer` (+ (* (- PlaybackPercent (`self.LastPercent`)) (`self.Duration`)) (`self.Timer`))))
  (set `self.LastPercent` PlaybackPercent)
  (if (> _output_get (`self.CD`))
    (set `self.Timer` 0.0)
    (if (> (`LoudnessNRT.GetNormalizedChannelLoudnessAtTime` (`self.LoudnessAnalyzer`) _returnvalue 0) (`LoudnessNRT.GetNormalizedChannelLoudnessAtTime` (`self.LoudnessAnalyzer`) (- _returnvalue 0.10132) 0))
      (goto _label))))

(fn `UserConstructionScript`
  (bind _sound (`AudioAnalyzerNRT.Sound` (`self.LoudnessAnalyzer`)))
  ;[1 1 1] Get Sound From Loudness Analyze
  (`AudioComponent.SetSound` (`self.Audio`) _sound)
  ;[1 1 1] Store Sound Duration
  (set `self.Duration` (`SoundBase.Duration` _sound)))