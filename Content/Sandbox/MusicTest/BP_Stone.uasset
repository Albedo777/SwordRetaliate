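; BP_Stone is a sandbox actor in the MusicTest folder that moves vertically and removes itself below ground zero.
; On BeginPlay it snaps to a fixed point above the world origin and flips 180 degrees.
; Each Tick it offsets its world Z by Speed scaled by delta time, without sweeping, and destroys itself once Z drops below zero.
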(event `self.ReceiveBeginPlay`
  (`self.K2_SetActorLocation` (0.0 0.0 500.0))
  (`self.K2_SetActorRotation` (struct :`Roll` 180.0)))

(event `self.ReceiveTick`
  (params (DeltaSeconds :type "Float (single-precision)"))
  (`self.K2_AddActorWorldOffset` (`KismetMathLibrary.MakeVector` 0.0 0.0 (* DeltaSeconds (`self.Speed`))))
  (if (< (.z (`self.K2_GetActorLocation`)) 0.0)
    (`self.K2_DestroyActor`)))

(fn `UserConstructionScript`)